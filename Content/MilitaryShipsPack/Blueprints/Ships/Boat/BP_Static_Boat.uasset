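; BP_Static_Boat is a boat Blueprint with a mounted gun, a cloaking field and a destroyed variant, built on a parent class.
; BeginPlay sets camera arm length, zoom limit and the destroyed class after the parent setup.
; Left mouse press and release activate and deactivate the child-actor gun by message, while V toggles cloaking on hull and gun.
; Tick copies rotator variables onto both engines' bases, rotators and screws.
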(event Custom|UpdateComponentsRotation
  ;[1 1 1] Update rotation
  (Transformation|SetRelativeRotation (Variables|Default|GetSM_Boat_L_Engine_Rotator) (Variables|Default|GetBoat_L_Engine_V_Rotator) false false)
  (Transformation|SetRelativeRotation (Variables|Default|GetSM_Boat_R_Engine_Rotator) (Variables|Default|GetBoat_R_Engine_V_Rotator) false false)
  (Transformation|SetRelativeRotation (Variables|Default|GetSM_Boat_R_Engine_Base) (Variables|Default|GetBoat_R_Engine_H_Rotator) false false)
  (Transformation|SetRelativeRotation (Variables|Default|GetSM_Boat_L_Engine_Base) (Variables|Default|GetBoat_L_Engine_H_Rotator) false false)
  (Transformation|SetRelativeRotation (Variables|Default|GetSM_L_Boat_Screw) (Variables|Default|GetBoat_L_Engine_Screw_Rotator) false false)
  (Transformation|SetRelativeRotation (Variables|Default|GetSM_R_Boat_Screw) (Variables|Default|GetBoat_R_Engine_Screw_Rotator) false false))

(event Custom|CloakGenerator
  ;[1 1 1] Cloaking field
  (CallFunction|ToggleCloakingField)
  (bind _asbp_boat_gun_01 (Utilities|Casting|CastToBP_Boat_Gun_01 (Variables|/Script/Engine.ChildActorComponent|GetChildActor (Variables|Default|GetBP_Boat_Gun_01)))
    (:then
      (Default|ToggleCloakingField _asbp_boat_gun_01))
    (:CastFailed
      (Development|PrintString "Can't cast to Gun 01"))))

(event EventTick
  (params (DeltaSeconds :type Float%20%28single-precision%29))
  ;[1 1 1] Update rotation
  (|CallParentFunction DeltaSeconds)
  (CallFunction|UpdateComponentsRotation))

(event EventBeginPlay
  ;[1 1 1] Set initial params
  (|CallParentFunction)
  (Variables|Default|SetDesiredArmLength 3e+03)
  (Variables|Default|SetMaxZoomIn 1e+03)
  (Variables|Default|SetDestroyedMesh "/Game/MilitaryShipsPack/Blueprints/Ships/Boat/BP_Boat_Destroyed.BP_Boat_Destroyed_C"))

(event Input|MouseEvents|LeftMouseButton
  (params (Key :type Key%20Structure :default "AnyKey"))
  ;[1 1 1] Fire gun
  (:Pressed
    (Class|BPModuleInterface|ActivateModule(Message) (Variables|/Script/Engine.ChildActorComponent|GetChildActor (Variables|Default|GetBP_Boat_Gun_01)) self))
  (:Released
    (Class|BPModuleInterface|DeactivateModule(Message) (Variables|/Script/Engine.ChildActorComponent|GetChildActor (Variables|Default|GetBP_Boat_Gun_01)))))

(event Input|KeyboardEvents|V
  (params (Key :type Key%20Structure :default "AnyKey"))
  ;[1 1 1] Cloaking field
  (:Pressed
    (CallFunction|CloakGenerator)))

(fn ConstructionScript
  (|CallParentFunction))