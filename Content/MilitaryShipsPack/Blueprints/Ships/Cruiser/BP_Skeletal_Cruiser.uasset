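; Player-controlled skeletal-mesh cruiser ship, a child Blueprint that adds gun input and ship-specific settings to its parent ship class.
; Left and right mouse buttons fire guns 01 and 02, each spawning a strike-pointer projectile at its barrel socket with an attached, enlarged muzzle-flash emitter.
; The V key toggles the cloaking field.
; BeginPlay sets the desired camera arm length and destroyed-cruiser replacement after running parent logic.
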(event EventBeginPlay
  ;[1 1 1] Set initial params
  (|CallParentFunction)
  (Variables|Default|SetDesiredArmLength 1.2e+04)
  (Variables|Default|SetDestroyedMesh "/Game/MilitaryShipsPack/Blueprints/Ships/Cruiser/BP_Cruiser_Destroyed.BP_Cruiser_Destroyed_C"))

(event EventTick
  (params (DeltaSeconds :type Float%20%28single-precision%29))
  ;[1 1 1] Event tick
  (|CallParentFunction DeltaSeconds))

(event Input|MouseEvents|LeftMouseButton
  (params (Key :type Key%20Structure :default "AnyKey"))
  ;[1 1 1] Fire gun 01
  (:Pressed
    (Game|SpawnActorfromClass "/Game/MilitaryShipsPack/Blueprints/Projectiles/BP_GunProjectileStrikePointer.BP_GunProjectileStrikePointer_C" (Transformation|GetSocketTransform (Variables|Default|GetSK_Cruiser) "Gun_01_BarrelSocket" "RTS_World") "Undefined" 0 self 0)
    (bind _returnvalue (Effects|SpawnEmitterAttached "/Game/MilitaryShipsPack/Particles/PS_Gun_Fire.PS_Gun_Fire" (Variables|Default|GetSK_Cruiser) "Gun_01_BarrelSocket" "200.000000, 0, 0"))
    (Transformation|SetRelativeScale3D _returnvalue "2.000000,2.000000,2.000000")))

(event Input|MouseEvents|RightMouseButton
  (params (Key :type Key%20Structure :default "AnyKey"))
  ;[1 1 1] Fire gun 02
  (:Pressed
    (Game|SpawnActorfromClass "/Game/MilitaryShipsPack/Blueprints/Projectiles/BP_GunProjectileStrikePointer.BP_GunProjectileStrikePointer_C" (Transformation|GetSocketTransform (Variables|Default|GetSK_Cruiser) "Gun_02_BarrelSocket" "RTS_World") "Undefined" 0 self 0)
    (bind _returnvalue (Effects|SpawnEmitterAttached "/Game/MilitaryShipsPack/Particles/PS_Gun_Fire.PS_Gun_Fire" (Variables|Default|GetSK_Cruiser) "Gun_02_BarrelSocket" "200.000000, 0, 0"))
    (Transformation|SetRelativeScale3D _returnvalue "2.000000,2.000000,2.000000")))

(event Input|KeyboardEvents|V
  (params (Key :type Key%20Structure :default "AnyKey"))
  ;[1 1 1] Cloaking field
  (:Pressed
    (CallFunction|ToggleCloakingField)))

(fn ConstructionScript
  (|CallParentFunction))