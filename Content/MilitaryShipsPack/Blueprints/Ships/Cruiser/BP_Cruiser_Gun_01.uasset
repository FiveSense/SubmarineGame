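; Cruiser gun module Blueprint for the military ships pack, with a rotating base and barrel that fires when activated.
; Activation stores the activator, spawns a projectile strike pointer at the barrel socket with it as initiator, and attaches an enlarged muzzle-fire particle effect.
; Every tick it applies the base and barrel rotation variables to their meshes; this graph does not compute those rotations.
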(event Custom|UpdateComponentsRotation
  ;[1 1 1] Update rotation
  (Transformation|SetRelativeRotation (Variables|Default|GetSM_Cruiser_Gun_Base) (Variables|Default|GetGunBaseRotation) false false)
  (Transformation|SetRelativeRotation (Variables|Default|GetSM_Cruiser_Gun_Barrel) (Variables|Default|GetGunBarrelRotation) false false))

(event EventActivateModule
  (params (Activator :type BP%20Ship%20Base%20Object%20Reference))
  ;[1 1 1] Activate
  (Variables|Default|SetActivator Activator)
  (Game|SpawnActorfromClass "/Game/MilitaryShipsPack/Blueprints/Projectiles/BP_GunProjectileStrikePointer.BP_GunProjectileStrikePointer_C" (Transformation|GetSocketTransform (Variables|Default|GetSM_Cruiser_Gun_Barrel) "Gun_01_Socket" "RTS_World") "Undefined" 0 (Variables|Default|GetActivator) 0)
  (bind _returnvalue (Effects|SpawnEmitterAttached "/Game/MilitaryShipsPack/Particles/PS_Gun_Fire.PS_Gun_Fire" (Variables|Default|GetSM_Cruiser_Gun_Barrel) "Gun_01_Socket" "200.000000, 0, 0"))
  (Transformation|SetRelativeScale3D _returnvalue "2.000000,2.000000,2.000000"))

(event EventTick
  (params (DeltaSeconds :type Float%20%28single-precision%29))
  ;[1 1 1] Update rotation
  (CallFunction|UpdateComponentsRotation))

(fn ConstructionScript
  (|CallParentFunction))