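; Static cruiser ship Blueprint that extends a parent ship class with two gun child actors, a rotating radar and a test cloaking field.
; Left and right mouse buttons send an activate-module message to guns 01 and 02 respectively.
; The V key toggles cloaking on the hull, then on both guns through casts.
; BeginPlay sets arm length and destroyed mesh, while Tick applies the radar rotation.
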(event Custom|UpdateComponentsRotation
  ;[1 1 1] Update rotation
  (Transformation|SetRelativeRotation (Variables|Default|GetSM_Radar) (Variables|Default|GetRadarRotation) false false))

(event Custom|CloakGenerator
  ;[1 1 1] Cloaking field test
  (CallFunction|ToggleCloakingField)
  (bind _asbp_cruiser_gun_01 (Utilities|Casting|CastToBP_Cruiser_Gun_01 (Variables|/Script/Engine.ChildActorComponent|GetChildActor (Variables|Default|GetBP_Cruiser_Gun_01)))
    (:then
      (Default|ToggleCloakingField _asbp_cruiser_gun_01)
      (bind _asbp_cruiser_gun_02 (Utilities|Casting|CastToBP_Cruiser_Gun_02 (Variables|/Script/Engine.ChildActorComponent|GetChildActor (Variables|Default|GetBP_Cruiser_Gun_02)))
        (:then
          (Default|ToggleCloakingField _asbp_cruiser_gun_02))
        (:CastFailed
          (Development|PrintString "Can't cast to Cruiser Gun 02"))))
    (:CastFailed
      (Development|PrintString "Can't cast to Cruiser Gun 01"))))

(event EventTick
  (params (DeltaSeconds :type Float%20%28single-precision%29))
  ;[1 1 1] Update rotation
  (|CallParentFunction DeltaSeconds)
  (CallFunction|UpdateComponentsRotation))

(event EventBeginPlay
  ;[1 1 1] Set initial params
  (|CallParentFunction)
  (Variables|Default|SetDesiredArmLength 1.2e+04)
  (Variables|Default|SetDestroyedMesh "/Game/MilitaryShipsPack/Blueprints/Ships/Cruiser/BP_Cruiser_Destroyed.BP_Cruiser_Destroyed_C"))

(event Input|MouseEvents|LeftMouseButton
  (params (Key :type Key%20Structure :default "AnyKey"))
  ;[1 1 1] Fire gun 01
  (:Pressed
    (Class|BPModuleInterface|ActivateModule(Message) (Variables|/Script/Engine.ChildActorComponent|GetChildActor (Variables|Default|GetBP_Cruiser_Gun_01)) self)))

(event Input|MouseEvents|RightMouseButton
  (params (Key :type Key%20Structure :default "AnyKey"))
  ;[1 1 1] Fire gun 02
  (:Pressed
    (Class|BPModuleInterface|ActivateModule(Message) (Variables|/Script/Engine.ChildActorComponent|GetChildActor (Variables|Default|GetBP_Cruiser_Gun_02)) self)))

(event Input|KeyboardEvents|V
  (params (Key :type Key%20Structure :default "AnyKey"))
  ;[1 1 1] Cloaking field test
  (:Pressed
    (CallFunction|CloakGenerator)))

(fn ConstructionScript
  (|CallParentFunction))