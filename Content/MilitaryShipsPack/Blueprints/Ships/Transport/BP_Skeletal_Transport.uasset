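; Player-controllable transport ship Blueprint that adds weapons and setup on top of a parent ship class.
; Right mouse spawns homing missiles from both rocket turret sockets, while left mouse spawns a gun projectile with an attached muzzle effect.
; BeginPlay sets the camera arm length and destroyed-ship class, and V toggles the cloaking field.
; Tick and construction only call the parent.
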(event EventBeginPlay
  ;[1 1 1] Set initial params
  (|CallParentFunction)
  (Variables|Default|SetDesiredArmLength 1.4e+04)
  (Variables|Default|SetDestroyedMesh "/Game/MilitaryShipsPack/Blueprints/Ships/Transport/BP_Transport_Destroyed.BP_Transport_Destroyed_C"))

(event EventTick
  (params (DeltaSeconds :type Float%20%28single-precision%29))
  ;[1 1 1] Event tick
  (|CallParentFunction DeltaSeconds))

(event Input|MouseEvents|LeftMouseButton
  (params (Key :type Key%20Structure :default "AnyKey"))
  ;[1 1 1] Fire gun 01
  (:Pressed
    (Game|SpawnActorfromClass "/Game/MilitaryShipsPack/Blueprints/Projectiles/BP_GunProjectileStrikePointer.BP_GunProjectileStrikePointer_C" (Transformation|GetSocketTransform (Variables|Default|GetSK_Transport) "Gun_BarrelSocket" "RTS_World") "Undefined" 0 self 0)
    (bind _returnvalue (Effects|SpawnEmitterAttached "/Game/MilitaryShipsPack/Particles/PS_Gun_Fire.PS_Gun_Fire" (Variables|Default|GetSK_Transport) "Gun_BarrelSocket" "50.000000, 0, 0"))
    (Transformation|SetRelativeScale3D _returnvalue "1.000000,1.000000,1.000000")))

(event Input|MouseEvents|RightMouseButton
  (params (Key :type Key%20Structure :default "AnyKey"))
  ;[1 1 1] Fire rockets
  (:Pressed
    (Game|SpawnActorfromClass "/Game/MilitaryShipsPack/Blueprints/Projectiles/BP_HomingMissileProjectile.BP_HomingMissileProjectile_C" (Transformation|GetSocketTransform (Variables|Default|GetSK_Transport) "Rocket_Turret_L_BarrelSocket" "RTS_World") "Undefined" 0 self 0)
    (Game|SpawnActorfromClass "/Game/MilitaryShipsPack/Blueprints/Projectiles/BP_HomingMissileProjectile.BP_HomingMissileProjectile_C" (Transformation|GetSocketTransform (Variables|Default|GetSK_Transport) "Rocket_Turret_R_BarrelSocket" "RTS_World") "Undefined" 0 self 0)))

(event Input|KeyboardEvents|V
  (params (Key :type Key%20Structure :default "AnyKey"))
  ;[1 1 1] Cloaking field
  (:Pressed
    (CallFunction|ToggleCloakingField)))

(fn ConstructionScript
  (|CallParentFunction))