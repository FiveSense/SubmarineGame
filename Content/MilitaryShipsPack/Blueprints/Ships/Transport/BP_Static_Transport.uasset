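; Transport ship Blueprint built on a parent ship class, with a gun, left and right rocket turrets and twin screws.
; Left mouse fires the gun and right mouse both turrets, by messaging their child actors.
; V toggles the cloaking field on the hull, then on each weapon through chained casts.
; BeginPlay sets camera arm length and destroyed mesh, while Tick applies screw rotations.
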(event Custom|UpdateComponentsRotation
  ;[1 1 1] Update rotation
  (Transformation|SetRelativeRotation (Variables|Default|GetSM_Transport_Screw_R) (Variables|Default|GetScrew_R_Rotation) false false)
  (Transformation|SetRelativeRotation (Variables|Default|GetSM_Transport_Screw_L) (Variables|Default|GetScrew_L_Rotation) false false))

(event Custom|CloakGenerator
  ;[1 1 1] Cloaking field test
  (CallFunction|ToggleCloakingField)
  (bind _asbp_transport_gun_01 (Utilities|Casting|CastToBP_Transport_Gun_01 (Variables|/Script/Engine.ChildActorComponent|GetChildActor (Variables|Default|GetBP_Transport_Gun_01)))
    (:then
      (Default|ToggleCloakingField _asbp_transport_gun_01)
      (bind _asbp_transport_rocket_turret_01 (Utilities|Casting|CastToBP_Transport_Rocket_Turret_01 (Variables|/Script/Engine.ChildActorComponent|GetChildActor (Variables|Default|GetBP_Transport_Rocket_Turret_L)))
        (:then
          (Default|ToggleCloakingField _asbp_transport_rocket_turret_01)
          (bind _asbp_transport_rocket_turret_01_2 (Utilities|Casting|CastToBP_Transport_Rocket_Turret_01 (Variables|/Script/Engine.ChildActorComponent|GetChildActor (Variables|Default|GetBP_Transport_Rocket_Turret_R)))
            (:then
              (Default|ToggleCloakingField _asbp_transport_rocket_turret_01_2))
            (:CastFailed
              (Development|PrintString "Can't cast to Rocket Turret"))))
        (:CastFailed
          (Development|PrintString "Can't cast to Rocket Turret"))))
    (:CastFailed
      (Development|PrintString "Can't cast to Transport Gun 01"))))

(event EventTick
  (params (DeltaSeconds :type Float%20%28single-precision%29))
  ;[1 1 1] Update rotation
  (|CallParentFunction DeltaSeconds)
  (CallFunction|UpdateComponentsRotation))

(event EventBeginPlay
  ;[1 1 1] Set initial params
  (|CallParentFunction)
  (Variables|Default|SetDesiredArmLength 1.4e+04)
  (Variables|Default|SetDestroyedMesh "/Game/MilitaryShipsPack/Blueprints/Ships/Transport/BP_Transport_Destroyed.BP_Transport_Destroyed_C"))

(event Input|MouseEvents|LeftMouseButton
  (params (Key :type Key%20Structure :default "AnyKey"))
  ;[1 1 1] Fire gun 01
  (:Pressed
    (Class|BPModuleInterface|ActivateModule(Message) (Variables|/Script/Engine.ChildActorComponent|GetChildActor (Variables|Default|GetBP_Transport_Gun_01)) self)))

(event Input|MouseEvents|RightMouseButton
  (params (Key :type Key%20Structure :default "AnyKey"))
  ;[1 1 1] Fire rockets
  (:Pressed
    (Class|BPModuleInterface|ActivateModule(Message) (Variables|/Script/Engine.ChildActorComponent|GetChildActor (Variables|Default|GetBP_Transport_Rocket_Turret_L)) self)
    (Class|BPModuleInterface|ActivateModule(Message) (Variables|/Script/Engine.ChildActorComponent|GetChildActor (Variables|Default|GetBP_Transport_Rocket_Turret_R)) self)))

(event Input|KeyboardEvents|V
  (params (Key :type Key%20Structure :default "AnyKey"))
  ;[1 1 1] Cloaking field test
  (:Pressed
    (CallFunction|CloakGenerator)))

(fn ConstructionScript
  (|CallParentFunction))