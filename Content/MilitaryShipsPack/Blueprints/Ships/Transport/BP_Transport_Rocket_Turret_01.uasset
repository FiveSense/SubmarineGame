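; Transport ship rocket turret module that fires homing missiles when activated.
; ActivateModule stores the activator and spawns a BP_HomingMissileProjectile at the barrel's rocket socket, passing the activator as initiator.
; Every tick it applies the base and barrel rotation variables to their meshes as relative rotations.
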(event Custom|UpdateComponentsRotation
  ;[1 1 1] Update rotation
  (Transformation|SetRelativeRotation (Variables|Default|GetSM_Transport_Rocket_Turret_Base) (Variables|Default|GetGunBaseRotation) false false)
  (Transformation|SetRelativeRotation (Variables|Default|GetSM_Transport_Rocket_Turret_Barrel) (Variables|Default|GetGunBarrelRotation) false false))

(event EventActivateModule
  (params (Activator :type BP%20Ship%20Base%20Object%20Reference))
  ;[1 1 1] Activate
  (Variables|Default|SetActivator Activator)
  (Game|SpawnActorfromClass "/Game/MilitaryShipsPack/Blueprints/Projectiles/BP_HomingMissileProjectile.BP_HomingMissileProjectile_C" (Transformation|GetSocketTransform (Variables|Default|GetSM_Transport_Rocket_Turret_Barrel) "Rocket_Socket" "RTS_World") "Undefined" 0 (Variables|Default|GetActivator) 0))

(event EventTick
  (params (DeltaSeconds :type Float%20%28single-precision%29))
  ;[1 1 1] Update rotation
  (CallFunction|UpdateComponentsRotation))

(fn ConstructionScript
  (|CallParentFunction))