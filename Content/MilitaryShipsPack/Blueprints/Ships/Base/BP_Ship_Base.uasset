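; BP_Ship_Base is the base ship pawn, handling health, collision damage, destruction, cloaking and camera control.
; Hits apply radial damage plus point self-damage; at zero health it spawns explosion effects and DestroyedMesh, then destroys itself.
; A timeline drives material Dissolve for cloaking, and input controls free camera, Tick-smoothed spring-arm zoom and hold-to-slow time.
; Getter functions expose dead, enemy and visibility flags, while component getters return nothing.
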(event Custom|ToggleCloakingField
  ;[1 1 1] Toggle cloaking field
  (if (Variables|Modules|GetIsCloakingFieldActive)
    (Variables|Modules|SetIsCloakingFieldActive false)
    (bind _dissolvevalue (Timeline|CloakingFieldAnimation Reverse)
      (:Update
        (CallFunction|CloakingField _dissolvevalue)))
    (else
      (Variables|Modules|SetIsCloakingFieldActive true)
      (Timeline|CloakingFieldAnimation Play))))

(event Custom|CloakingField
  (params (DissolveValue :type Float%20%28single-precision%29))
  ;[1 1 1] Cloaking Field
  (for _array_element (Variables|/Game/MilitaryShipsPack/Blueprints/Ships/Base/BP_MaterialController.BP_MaterialController_C|GetMaterials (Variables|Default|GetBP_MaterialController))
    (if (Utilities|IsValid _array_element)
      (Rendering|Material|SetScalarParameterValue _array_element "Dissolve" DissolveValue :!class /Script/Engine.MaterialInstanceDynamic))))

(event Collision|EventHit
  (params (MyComp :type Primitive%20Component%20Object%20Reference) (Other :type Actor%20Object%20Reference) (OtherComp :type Primitive%20Component%20Object%20Reference) (bSelfMoved :type Boolean) (HitLocation :type Vector) (HitNormal :type Vector) (NormalImpulse :type Vector) (Hit :type Hit%20Result%20Structure%20%28by%20ref%29))
  ;[1 1 1] Apply damage on hit
  (|CallParentFunction MyComp Other OtherComp bSelfMoved HitLocation HitNormal NormalImpulse Hit)
  (Utilities|Casting|CastToBP_Ship_Base Other
    (:then
      (Class|GameplayStatics|ApplyRadialDamagewithFalloff (Variables|Damage|GetOtherShipImpactDamage) 1.0 HitLocation 1e+01 1e+02 1.0 "/Script/Engine.DamageType" 0 self (Pawn|GetController) "ECC_Visibility"))
    (:CastFailed
      (Class|GameplayStatics|ApplyRadialDamagewithFalloff Other 1.0 1.0 HitLocation 1e+01 1e+02 1.0 "/Script/Engine.DamageType" 0 self (Pawn|GetController) "ECC_Visibility")))
  (Game|Damage|ApplyPointDamage self (Variables|Damage|GetDamageToShipOnHit) NormalImpulse Hit 0 0 "/Script/Engine.DamageType"))

(event EventTick
  (params (DeltaSeconds :type Float%20%28single-precision%29))
  ;[1 1 1] Smooth camera zoom
  (Utilities|FlowControl|Sequence
    (:then_0
      (if (!= (Variables|/Script/Engine.SpringArmComponent|GetTargetArmLength (Variables|Default|GetSpringArm)) (Variables|Camera|GetDesiredArmLength))
        (Variables|/Script/Engine.SpringArmComponent|SetTargetArmLength (Variables|Default|GetSpringArm) (Math|Float|Clamp(Float) (Math|Interpolation|FInterpTo (Variables|/Script/Engine.SpringArmComponent|GetTargetArmLength (Variables|Default|GetSpringArm)) (Variables|Camera|GetDesiredArmLength) (Utilities|Time|GetWorldDeltaSeconds) 5.0) (Variables|Camera|GetMaxZoomIn) (Variables|Camera|GetMaxZoomOut)))))))

(event Game|Damage|EventAnyDamage
  (params (Damage :type Float%20%28single-precision%29) (DamageType :type Damage%20Type%20Object%20Reference) (InstigatedBy :type Controller%20Object%20Reference) (DamageCauser :type Actor%20Object%20Reference))
  (bind _returnvalue (Transformation|GetActorLocation))
  ;[1 1 1] Apply damage and destroy ship
  (Variables|Damage|SetCurrentHealth (- (Variables|Damage|GetCurrentHealth) Damage))
  (if (<= (Variables|Damage|GetCurrentHealth) 0.0)
    (Utilities|FlowControl|DoOnce false
      (:Completed
        (Audio|PlaySoundatLocation "/Game/MilitaryShipsPack/Sounds/Common/SC_Explosion_01_Cue.SC_Explosion_01_Cue" _returnvalue)
        (bind _returnvalue_2 (Effects|SpawnEmitteratLocation "/Game/MilitaryShipsPack/Particles/PS_ExplosionWithShrapnel.PS_ExplosionWithShrapnel" _returnvalue))
        (Transformation|SetRelativeScale3D _returnvalue_2 "15.000000,15.000000,15.000000")
        (Game|SpawnActorfromClass (Variables|Damage|GetDestroyedMesh) (Transformation|GetActorTransform) "AlwaysSpawn" 0 0)
        (Actor|DestroyActor)))))

(event EventBeginPlay
  ;[1 1 1] Set current health
  (Variables|Damage|SetCurrentHealth (Variables|Damage|GetInitialHealth)))

(event Input|AxisEvents|InputAxisCameraYaw
  (params (AxisValue :type Float%20%28single-precision%29))
  ;[1 1 1] Free camera movement
  (Pawn|Input|AddControllerYawInput (* AxisValue 4e+01 (Utilities|Time|GetWorldDeltaSeconds))))

(event Input|AxisEvents|InputAxisCameraPitch
  (params (AxisValue :type Float%20%28single-precision%29))
  (bind _returnvalue (Game|GetPlayerController 0))
  (bind _returnvalue_2 (Pawn|GetControlRotation _returnvalue :!class /Script/Engine.Controller))
  (bind (_roll _pitch _yaw) (Math|Rotator|BreakRotator _returnvalue_2))
  ;[1 1 1] Free camera movement
  (Pawn|SetControlRotation (Game|GetPlayerController 0) (Math|Rotator|MakeRotator _roll (+ (Math|Float|ClampAngle (- (+ (* AxisValue 4e+01 (Utilities|Time|GetWorldDeltaSeconds)) _pitch) 1.8e+02) 1.2e+02 -1.8e+02) 1.8e+02) _yaw)))

(event Input|KeyboardEvents|C
  (params (Key :type Key%20Structure :default "AnyKey"))
  (bind _springarm (Variables|Default|GetSpringArm))
  (bind _springarm_2 (Variables|Default|GetSpringArm))
  ;[1 1 1] Enable/Disable Free Camera
  (:Pressed
    (if (Variables|Camera|GetIsFreeCameraEnabled)
      (Variables|Camera|SetIsFreeCameraEnabled false)
      (Variables|/Script/Engine.SpringArmComponent|SetbUsePawnControlRotation _springarm_2 false)
      (Variables|/Script/Engine.SpringArmComponent|SetCameraRotationLagSpeed _springarm_2 3.0)
      (Transformation|SetRelativeRotation _springarm_2 "-20.000000, 0, 0" false false)
      (else
        (Variables|Camera|SetIsFreeCameraEnabled true)
        (Variables|/Script/Engine.SpringArmComponent|SetbUsePawnControlRotation _springarm true)
        (Variables|/Script/Engine.SpringArmComponent|SetCameraRotationLagSpeed _springarm 8.0)
        (Pawn|Input|AddControllerPitchInput 2e+01)))))

(event Input|MouseEvents|MouseWheelUp
  (params (Key :type Key%20Structure :default "AnyKey"))
  ;[1 1 1] Camera zoom
  (:Pressed
    (Variables|Camera|SetDesiredArmLength (Math|Float|Clamp(Float) (- (Variables|/Script/Engine.SpringArmComponent|GetTargetArmLength (Variables|Default|GetSpringArm)) (Variables|Camera|GetCameraSensitivity)) (Variables|Camera|GetMaxZoomIn) (Variables|Camera|GetMaxZoomOut)))))

(event Input|MouseEvents|MouseWheelDown
  (params (Key :type Key%20Structure :default "AnyKey"))
  ;[1 1 1] Camera zoom
  (:Pressed
    (Variables|Camera|SetDesiredArmLength (Math|Float|Clamp(Float) (+ (Variables|/Script/Engine.SpringArmComponent|GetTargetArmLength (Variables|Default|GetSpringArm)) (Variables|Camera|GetCameraSensitivity)) (Variables|Camera|GetMaxZoomIn) (Variables|Camera|GetMaxZoomOut)))))

(event Input|KeyboardEvents|Z
  (params (Key :type Key%20Structure :default "AnyKey"))
  ;[1 1 1] Slow Mo
  (:Pressed
    (Utilities|Time|SetGlobalTimeDilation 0.1))
  (:Released
    (Utilities|Time|SetGlobalTimeDilation 1.0)))

(fn ConstructionScript)

(fn GetCapsuleCollision
  (return 0))

(fn GetSkeletalMesh
  (return 0))

(fn GetStaticMesh
  (return 0))

(fn IsDead
  (return (Variables|Damage|GetIsShipDead)))

(fn IsEnemyforPlayer
  (return (Variables|AI|GetIsEnemyShip)))

(fn IsVisibleforEnemies
  (return (Variables|Common|GetIsShipVisible)))