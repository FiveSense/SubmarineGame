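; Actor component for military ships that manages dynamic materials so the owner can switch to a destroyed look.
; On BeginPlay it creates dynamic instances for the owner's skeletal and static meshes, plus child-actor modules queried through BP_ModuleInterface, and caches them.
; AddSkeletalMesh registers further meshes the same way.
; ApplyDestroyedMaterial sets fixed dissolve, darkening, roughness and emissive parameters on every cached instance, ignoring its DissolveValue input.
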(event Custom|GetStaticMeshes
  ;[1 1 1] Get Static Meshes
  (for _array_element (Actor|GetComponentsByClass (Components|GetOwner) "/Script/Engine.StaticMeshComponent")
    (for (_array_element_2 _array_index) (Rendering|Material|GetMaterials _array_element)
      (bind _returnvalue (Rendering|Material|CreateDynamicMaterialInstance _array_element_2 :!class /Script/Engine.KismetMaterialLibrary))
      (Rendering|Material|SetMaterial _array_element _array_index _returnvalue)
      (Utilities|Array|Add (Variables|Default|GetMaterials) _returnvalue))))

(event Custom|AddSkeletalMesh
  (params (SkeletalMesh :type Skeletal%20Mesh%20Component%20Object%20Reference))
  ;[1 1 1] Add Skeletal Mesh
  (for (_array_element _array_index) (Rendering|Material|GetMaterials SkeletalMesh)
    (bind _returnvalue (Rendering|Material|CreateDynamicMaterialInstance _array_element :!class /Script/Engine.KismetMaterialLibrary))
    (Rendering|Material|SetMaterial SkeletalMesh _array_index _returnvalue)
    (Utilities|Array|Add (Variables|Default|GetMaterials) _returnvalue)))

(event Custom|GetSkeletalMeshes
  ;[1 1 1] Get Skeletal Meshes
  (for _array_element (Actor|GetComponentsByClass (Components|GetOwner) "/Script/Engine.SkeletalMeshComponent")
    (for (_array_element_2 _array_index) (Rendering|Material|GetMaterials _array_element)
      (bind _returnvalue (Rendering|Material|CreateDynamicMaterialInstance _array_element_2 :!class /Script/Engine.KismetMaterialLibrary))
      (Rendering|Material|SetMaterial _array_element _array_index _returnvalue)
      (Utilities|Array|Add (Variables|Default|GetMaterials) _returnvalue))))

(event Custom|GetModules
  ;[1 1 1] Get Modules
  (for _array_element (Actor|GetComponentsByClass (Components|GetOwner) "/Script/Engine.ChildActorComponent")
    (if (Utilities|DoesObjectImplementInterface (Variables|/Script/Engine.ChildActorComponent|GetChildActor _array_element) "/Game/MilitaryShipsPack/Blueprints/Common/BP_ModuleInterface.BP_ModuleInterface_C")
      ;;[1 1 1] Get skeletal meshes
      (bind _skeletalmesh (Class|BPModuleInterface|GetSkeletalMesh(Message) (Variables|/Script/Engine.ChildActorComponent|GetChildActor _array_element)))
      (if (== _skeletalmesh 0)
        ;;[1 1 1] Get static meshes
        (bind _staticmesh (Class|BPModuleInterface|GetStaticMesh(Message) (Variables|/Script/Engine.ChildActorComponent|GetChildActor _array_element)))
        (if (!= _staticmesh 0)
          (for (_array_element_2 _array_index) (Rendering|Material|GetMaterials _staticmesh)
            (bind _returnvalue (Rendering|Material|CreateDynamicMaterialInstance _array_element_2 :!class /Script/Engine.KismetMaterialLibrary))
            (Rendering|Material|SetMaterial _staticmesh _array_index _returnvalue)
            (Utilities|Array|Add (Variables|Default|GetMaterials) _returnvalue)))
        (else
          (for (_array_element_3 _array_index_2) (Rendering|Material|GetMaterials _skeletalmesh)
            (bind _returnvalue_2 (Rendering|Material|CreateDynamicMaterialInstance _array_element_3 :!class /Script/Engine.KismetMaterialLibrary))
            (Rendering|Material|SetMaterial _skeletalmesh _array_index_2 _returnvalue_2)
            (Utilities|Array|Add (Variables|Default|GetMaterials) _returnvalue_2)))))))

(event Custom|ApplyDestroyedMaterial
  (params (DissolveValue :type Float%20%28single-precision%29))
  ;[1 1 1] Apply destroyed material
  (for _array_element (Variables|Default|GetMaterials)
    (if (Utilities|IsValid _array_element)
      (Rendering|Material|SetScalarParameterValue _array_element "Dissolve" 0.43 :!class /Script/Engine.MaterialInstanceDynamic)
      (Rendering|Material|SetScalarParameterValue _array_element "DissolveStrenght" 0.0 :!class /Script/Engine.MaterialInstanceDynamic)
      (Rendering|Material|SetVectorParameterValue :self _array_element :ParameterName "ColorMultiplier" :!class /Script/Engine.MaterialInstanceDynamic)
      (Rendering|Material|SetScalarParameterValue _array_element "RoughnessMultiplier" 3.0 :!class /Script/Engine.MaterialInstanceDynamic)
      (Rendering|Material|SetScalarParameterValue _array_element "EmissiveValue" 0.0 :!class /Script/Engine.MaterialInstanceDynamic)
      (Rendering|Material|SetVectorParameterValue :self _array_element :ParameterName "ColorMultiplierWithCamouflage" :!class /Script/Engine.MaterialInstanceDynamic))))

(event EventBeginPlay
  ;[1 1 1] Init component
  (CallFunction|GetSkeletalMeshes)
  (CallFunction|GetStaticMeshes)
  (CallFunction|GetModules))

(fn GetParent
  (return 0))

(fn GetSkeletalMesh
  (return 0))

(fn GetStaticMesh
  (return 0))