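; BP_Gun_Base is a base Blueprint for ship guns that provides a toggleable cloaking-field effect.
; Toggling flips the active flag and plays or reverses the CloakingFieldAnimation timeline, whose updates feed a dissolve value to CloakingField.
; CloakingField writes that value to the Dissolve scalar parameter on every valid material held by BPMaterialController.
; The parent, skeletal mesh and static mesh getters are empty stubs, and the construction script does nothing.
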(event Custom|ToggleCloakingField
  ;[1 1 1] Toggle cloaking field
  (if (Variables|Default|GetIsCloakingFieldActive)
    (Variables|Default|SetIsCloakingFieldActive false)
    (bind _dissolvevalue (Timeline|CloakingFieldAnimation Reverse)
      (:Update
        (CallFunction|CloakingField _dissolvevalue)))
    (else
      (Variables|Default|SetIsCloakingFieldActive true)
      (Timeline|CloakingFieldAnimation Play))))

(event Custom|CloakingField
  (params (DissolveValue :type Float%20%28single-precision%29))
  ;[1 1 1] Cloaking Field
  (for _array_element (Variables|/Game/MilitaryShipsPack/Blueprints/Ships/Base/BP_MaterialController.BP_MaterialController_C|GetMaterials (Variables|Default|GetBP_MaterialController))
    (if (Utilities|IsValid _array_element)
      (Rendering|Material|SetScalarParameterValue _array_element "Dissolve" DissolveValue :!class /Script/Engine.MaterialInstanceDynamic))))

(fn ConstructionScript)

(fn GetParent
  (return 0))

(fn GetSkeletalMesh
  (return 0))

(fn GetStaticMesh
  (return 0))