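; Player-controllable submarine ship Blueprint with two gun child actors, built on a parent ship class that it extends at BeginPlay and Tick.
; Left and right mouse buttons send an activate message to gun 01 and gun 02.
; V toggles a test cloaking field on the hull and both guns through casts.
; Each tick applies stored rotations to the fins and twin screws, and BeginPlay sets camera arm length and the destroyed mesh.
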(event Custom|UpdateComponentsRotation
  ;[1 1 1] Update rotation
  (Transformation|SetRelativeRotation (Variables|Default|GetSM_Submarine_Rear_Fin) (Variables|Default|GetRear_Fin_Rotation) false false)
  (Transformation|SetRelativeRotation (Variables|Default|GetSM_Submarine_Front_Fin_R) (Variables|Default|GetFront_Fin_R_Rotation) false false)
  (Transformation|SetRelativeRotation (Variables|Default|GetSM_Submarine_Front_Fin_L) (Variables|Default|GetFront_Fin_L_Rotation) false false)
  (Transformation|SetRelativeRotation (Variables|Default|GetSM_Submarine_Screw_R) (Variables|Default|GetScrew_R_Rotation) false false)
  (Transformation|SetRelativeRotation (Variables|Default|GetSM_Submarine_Screw_L) (Variables|Default|GetScrew_L_Rotation) false false))

(event Custom|CloakGenerator
  ;[1 1 1] Cloaking field test
  (CallFunction|ToggleCloakingField)
  (bind _asbp_submarine_gun_01 (Utilities|Casting|CastToBP_Submarine_Gun_01 (Variables|/Script/Engine.ChildActorComponent|GetChildActor (Variables|Default|GetBP_Submarine_Gun_01)))
    (:then
      (Default|ToggleCloakingField _asbp_submarine_gun_01)
      (bind _asbp_submarine_gun_02 (Utilities|Casting|CastToBP_Submarine_Gun_02 (Variables|/Script/Engine.ChildActorComponent|GetChildActor (Variables|Default|GetBP_Submarine_Gun_02)))
        (:then
          (Default|ToggleCloakingField _asbp_submarine_gun_02))
        (:CastFailed
          (Development|PrintString "Can't cast to Submarine Gun 02"))))
    (:CastFailed
      (Development|PrintString "Can't cast to Submarine Gun 01"))))

(event EventTick
  (params (DeltaSeconds :type Float%20%28single-precision%29))
  ;[1 1 1] Update rotation
  (|CallParentFunction DeltaSeconds)
  (CallFunction|UpdateComponentsRotation))

(event EventBeginPlay
  ;[1 1 1] Set initial params
  (|CallParentFunction)
  (Variables|Default|SetDesiredArmLength 1.1e+04)
  (Variables|Default|SetDestroyedMesh "/Game/MilitaryShipsPack/Blueprints/Ships/Submarine/BP_Submarine_Destroyed.BP_Submarine_Destroyed_C"))

(event Input|MouseEvents|LeftMouseButton
  (params (Key :type Key%20Structure :default "AnyKey"))
  ;[1 1 1] Fire gun 01
  (:Pressed
    (Class|BPModuleInterface|ActivateModule(Message) (Variables|/Script/Engine.ChildActorComponent|GetChildActor (Variables|Default|GetBP_Submarine_Gun_01)) self)))

(event Input|MouseEvents|RightMouseButton
  (params (Key :type Key%20Structure :default "AnyKey"))
  ;[1 1 1] Fire gun 02
  (:Pressed
    (Class|BPModuleInterface|ActivateModule(Message) (Variables|/Script/Engine.ChildActorComponent|GetChildActor (Variables|Default|GetBP_Submarine_Gun_02)) self)))

(event Input|KeyboardEvents|V
  (params (Key :type Key%20Structure :default "AnyKey"))
  ;[1 1 1] Cloaking field test
  (:Pressed
    (CallFunction|CloakGenerator)))

(fn ConstructionScript
  (|CallParentFunction))