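; BP_Static_PatrolShip is a patrol ship child Blueprint with a gun child actor, a rotating part and a cloaking field test.
; BeginPlay sets the camera arm length and destroyed mesh on top of parent setup.
; Left mouse fires the gun via an activate-module message, and V toggles cloaking on both ship and gun.
; Tick applies RotatorRotation to the rotator mesh after parent Tick.
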(event Custom|UpdateComponentsRotation
  ;[1 1 1] Update rotation
  (Transformation|SetRelativeRotation (Variables|Default|GetSM_Patrol_Ship_Rotator) (Variables|Default|GetRotatorRotation) false false))

(event Custom|CloakGenerator
  ;[1 1 1] Cloaking field test
  (CallFunction|ToggleCloakingField)
  (bind _asbp_patrol_ship_gun (Utilities|Casting|CastToBP_Patrol_Ship_Gun (Variables|/Script/Engine.ChildActorComponent|GetChildActor (Variables|Default|GetBP_PatrolShip_Gun_01)))
    (:then
      (Default|ToggleCloakingField _asbp_patrol_ship_gun))
    (:CastFailed
      (Development|PrintString "Can't cast to Gun 01"))))

(event EventTick
  (params (DeltaSeconds :type Float%20%28single-precision%29))
  ;[1 1 1] Update rotation
  (|CallParentFunction DeltaSeconds)
  (CallFunction|UpdateComponentsRotation))

(event EventBeginPlay
  ;[1 1 1] Set initial params
  (|CallParentFunction)
  (Variables|Default|SetDesiredArmLength 6e+03)
  (Variables|Default|SetDestroyedMesh "/Game/MilitaryShipsPack/Blueprints/Ships/PatrolShip/BP_PatrolShip_Destroyed.BP_PatrolShip_Destroyed_C"))

(event Input|MouseEvents|LeftMouseButton
  (params (Key :type Key%20Structure :default "AnyKey"))
  ;[1 1 1] Fire gun 01
  (:Pressed
    (Class|BPModuleInterface|ActivateModule(Message) (Variables|/Script/Engine.ChildActorComponent|GetChildActor (Variables|Default|GetBP_PatrolShip_Gun_01)) self)))

(event Input|KeyboardEvents|V
  (params (Key :type Key%20Structure :default "AnyKey"))
  ;[1 1 1] Cloaking field test
  (:Pressed
    (CallFunction|CloakGenerator)))

(fn ConstructionScript
  (|CallParentFunction))