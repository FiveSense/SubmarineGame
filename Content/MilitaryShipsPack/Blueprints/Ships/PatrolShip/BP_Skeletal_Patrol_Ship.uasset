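; Player-controllable patrol ship Blueprint that specializes a parent ship class with its own gun, camera distance and destroyed version.
; Left mouse spawns a gun projectile strike pointer at the skeletal mesh's barrel socket and attaches a muzzle fire particle effect there.
; BeginPlay sets the desired arm length and destroyed mesh after calling the parent, which also handles tick and construction.
; The V key calls the cloaking field toggle.
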(event EventBeginPlay
  ;[1 1 1] Set initial params
  (|CallParentFunction)
  (Variables|Default|SetDesiredArmLength 6e+03)
  (Variables|Default|SetDestroyedMesh "/Game/MilitaryShipsPack/Blueprints/Ships/PatrolShip/BP_PatrolShip_Destroyed.BP_PatrolShip_Destroyed_C"))

(event EventTick
  (params (DeltaSeconds :type Float%20%28single-precision%29))
  ;[1 1 1] Event tick
  (|CallParentFunction DeltaSeconds))

(event Input|MouseEvents|LeftMouseButton
  (params (Key :type Key%20Structure :default "AnyKey"))
  ;[1 1 1] Fire gun 01
  (:Pressed
    (Game|SpawnActorfromClass "/Game/MilitaryShipsPack/Blueprints/Projectiles/BP_GunProjectileStrikePointer.BP_GunProjectileStrikePointer_C" (Transformation|GetSocketTransform (Variables|Default|GetSK_Patrol_Ship) "Gun_BarrelSocket" "RTS_World") "AlwaysSpawn" 0 self 0)
    (bind _returnvalue (Effects|SpawnEmitterAttached "/Game/MilitaryShipsPack/Particles/PS_Gun_Fire.PS_Gun_Fire" (Variables|Default|GetSK_Patrol_Ship) "Gun_BarrelSocket" "0.000000,50.000000,0.000000"))
    (Transformation|SetRelativeScale3D _returnvalue "1.000000,1.000000,1.000000")))

(event Input|KeyboardEvents|V
  (params (Key :type Key%20Structure :default "AnyKey"))
  ;[1 1 1] Cloaking field
  (:Pressed
    (CallFunction|ToggleCloakingField)))

(fn ConstructionScript
  (|CallParentFunction))