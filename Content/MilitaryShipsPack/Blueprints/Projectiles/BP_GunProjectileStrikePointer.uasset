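; BP_GunProjectileStrikePointer is a gun projectile that explodes on impact, or optionally after a set distance or time.
; It ignores its initiator in collision, plus the parent actor for player shots.
; A single-fire explosion triggers an impulse, explosion payload, impact decal and radial damage sparing the player, then destroys itself.
; An uncalled-here CalculateStrikePoint helper builds a downward-facing transform high above a target, with random positive XY offset.
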(event OnComponentHit(CollisionComponent)
  (params (HitComponent :type Primitive%20Component%20Object%20Reference) (OtherActor :type Actor%20Object%20Reference) (OtherComp :type Primitive%20Component%20Object%20Reference) (NormalImpulse :type Vector :default "0, 0, 0") (Hit :type Hit%20Result%20Structure%20%28by%20ref%29))
  (bind _explosionforce (Variables|Default|GetExplosionForce))
  ;[1 1 1] On hit or explode event
  (Utilities|FlowControl|DoOnce false
    (:Completed
      ;[1 1 1] Save hit result
      (Variables|Default|SetHitResult Hit)
      ;[1 1 1] Fire impulse
      (Class|RadialForceComponent|FireImpulse (Variables|Default|GetExplosionForce))
      ;[1 1 1] Execute payload
      (Default|Execute (Variables|Default|GetSimpleExplosionPayload_Big) (Transformation|GetWorldLocation (Variables|Default|GetExplosionForce)))
      ;[1 1 1] Save hit component
      (Variables|Default|SetHitComponent (.HitComponent (Collision|BreakHitResult (Variables|Default|GetHitResult))))
      ;[1 1 1] Spawn decal
      (Class|GameplayStatics|SpawnDecalAttached "/Game/MilitaryShipsPack/Materials/Bullet/M_Impact_Decal.M_Impact_Decal" "25.000000,25.000000,25.000000" (Variables|Default|GetHitComponent) "None" (.Location (Collision|BreakHitResult (Variables|Default|GetHitResult))) (Math|Conversions|RotationFromXVector (.Normal (Collision|BreakHitResult (Variables|Default|GetHitResult)))) "KeepWorldPosition" 6.0)
      ;[1 1 1] Apply damage
      (bind _pawn (Class|BPModuleInterface|GetParent(Message) (Game|Player|GetPlayerPawn 0)))
      (Game|Damage|ApplyRadialDamage (Variables|/Script/Engine.RadialForceComponent|GetDestructibleDamage _explosionforce) (Transformation|GetWorldLocation _explosionforce) (Variables|/Script/Engine.RadialForceComponent|GetRadius _explosionforce) "/Script/Engine.DamageType" (Utilities|Array|MakeArray (Game|Player|GetPlayerPawn 0) _pawn) self 0 false "ECC_Visibility")
      ;[1 1 1] Destroy projectile
      (Actor|DestroyActor))))

(event Custom|Explode
  (bind _explosionforce (Variables|Default|GetExplosionForce))
  ;[1 1 1] On hit or explode event
  (Utilities|FlowControl|DoOnce false
    (:Completed
      ;[1 1 1] Save hit result
      (Variables|Default|SetHitResult (stale OnComponentHit(CollisionComponent) Hit))
      ;[1 1 1] Fire impulse
      (Class|RadialForceComponent|FireImpulse (Variables|Default|GetExplosionForce))
      ;[1 1 1] Execute payload
      (Default|Execute (Variables|Default|GetSimpleExplosionPayload_Big) (Transformation|GetWorldLocation (Variables|Default|GetExplosionForce)))
      ;[1 1 1] Save hit component
      (Variables|Default|SetHitComponent (.HitComponent (Collision|BreakHitResult (Variables|Default|GetHitResult))))
      ;[1 1 1] Spawn decal
      (Class|GameplayStatics|SpawnDecalAttached "/Game/MilitaryShipsPack/Materials/Bullet/M_Impact_Decal.M_Impact_Decal" "25.000000,25.000000,25.000000" (Variables|Default|GetHitComponent) "None" (.Location (Collision|BreakHitResult (Variables|Default|GetHitResult))) (Math|Conversions|RotationFromXVector (.Normal (Collision|BreakHitResult (Variables|Default|GetHitResult)))) "KeepWorldPosition" 6.0)
      ;[1 1 1] Apply damage
      (bind _pawn (Class|BPModuleInterface|GetParent(Message) (Game|Player|GetPlayerPawn 0)))
      (Game|Damage|ApplyRadialDamage (Variables|/Script/Engine.RadialForceComponent|GetDestructibleDamage _explosionforce) (Transformation|GetWorldLocation _explosionforce) (Variables|/Script/Engine.RadialForceComponent|GetRadius _explosionforce) "/Script/Engine.DamageType" (Utilities|Array|MakeArray (Game|Player|GetPlayerPawn 0) _pawn) self 0 false "ECC_Visibility")
      ;[1 1 1] Destroy projectile
      (Actor|DestroyActor))))

(event EventBeginPlay
  ;[1 1 1] Check for initiator of projectile
  (if (== (Variables|Default|GetInitiator) (Game|Player|GetPlayerPawn 0))
    ;[1 1 1] Ignore player
    (Collision|IgnoreActorwhenMoving (Variables|Default|GetCollisionComponent) (Game|Player|GetPlayerPawn 0) true)
    (if (Utilities|DoesObjectImplementInterface (Game|Player|GetPlayerPawn 0) "/Game/MilitaryShipsPack/Blueprints/Common/BP_ModuleInterface.BP_ModuleInterface_C")
      (bind _pawn (Class|BPModuleInterface|GetParent(Message) (Game|Player|GetPlayerPawn 0)))
      (if (!= _pawn 0)
        (Collision|IgnoreActorwhenMoving (Variables|Default|GetCollisionComponent) _pawn true)))
    (else
      ;[1 1 1] Ignore initiator
      (Collision|IgnoreActorwhenMoving (Variables|Default|GetCollisionComponent) (Variables|Default|GetInitiator) true)))
  ;[1 1 1] Get start location
  (Variables|Default|SetStartLocation (Transformation|GetWorldLocation (Variables|Default|GetCollisionComponent)))
  ;[1 1 1] Explode after specified amount of time
  (if (Variables|Default|GetUseExplodeTime)
    (Utilities|FlowControl|Delay (Variables|Default|GetExplodeTime))
    (CallFunction|Explode)))

(event EventTick
  (params (DeltaSeconds :type Float%20%28single-precision%29))
  ;[1 1 1] Explode after specified amount of distance
  (if (Variables|Default|GetUseExplodeDistance)
    (if (>= (Math|Vector|VectorLength (- (Transformation|GetWorldLocation (Variables|Default|GetCollisionComponent)) (Variables|Default|GetStartLocation))) (Variables|Default|GetExplodeDistance))
      (CallFunction|Explode))))

(fn ConstructionScript)

(fn CalculateStrikePoint
  (params (StrikePoint :type Vector))
  (return (Math|Transform|MakeTransform (+ StrikePoint (Math|Vector|MakeVector (Math|Conversions|ToFloat(Integer) (Math|Random|RandomIntegerinRange 0 10000)) (Math|Conversions|ToFloat(Integer) (Math|Random|RandomIntegerinRange 0 10000)) 1e+05)) "-90.000000,0.000000,0.000000")))