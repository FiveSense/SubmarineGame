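; Player submarine pawn that registers with the game mode and constantly cruises forward, or descends once sunk.
; Each Tick it yaws toward the main camera's heading outside a small dead zone and updates its depth reading.
; Diving and surfacing teleport it behind camera fades, toggling buoyancy and hull glow.
; Aim mode swaps cameras and HUD crosshair while blocking dives; firing launches a missile at the first Ship found, if alive.
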(event Custom|Sunk
  (params (isSunk :type Boolean))
  ;[1 1 1] 沉没测试
  (Variables|Default|SetisSunk isSunk))

(event Custom|UpDown
  (params (isUp :type Boolean))
  (bind _returnvalue (Game|GetPlayerCameraManager 0))
  (bind _self self)
  (bind _self_2 self)
  (bind _buoyancy (Variables|Default|GetBuoyancy))
  (bind _returnvalue_2 (Transformation|GetActorLocation _self))
  (bind _returnvalue_3 (Transformation|GetActorLocation _self_2))
  ;[1 1 1] 潜艇上下潜
  (if (Variables|Default|GetisEnableUpDown)
    (bind _output_get (Variables|Default|SetisUp isUp))
    (if _output_get
      (Variables|Default|SetisEnableUpDown false)
      (CameraFades|StartCameraFade :self _returnvalue :ToAlpha 1.0 :Duration 2.0 :bShouldFadeAudio true :bHoldWhenFinished true)
      (Utilities|FlowControl|Delay 2.0)
      (Variables|/Game/PhysicalWaterSurface/Blueprints/Buoyancy.Buoyancy_C|SetEnableBuoyancy _buoyancy false)
      (Transformation|SetActorLocation _self (Math|Vector|MakeVector (.x _returnvalue_2) (.y _returnvalue_2) (- (.z _returnvalue_2) 5e+04)) false true)
      (Utilities|FlowControl|Delay 2.0)
      (CameraFades|StartCameraFade :self _returnvalue :FromAlpha 1.0 :Duration 2.0 :bShouldFadeAudio true :bHoldWhenFinished true)
      (Variables|Default|SetisEnableUpDown true)
      (Rendering|Material|SetScalarParameterValue (Variables|Default|GetSubMatInstance) "EmissiveValue" 5.0 :!class /Script/Engine.MaterialInstanceDynamic)
      (else
        (Variables|Default|SetisEnableUpDown false)
        (CameraFades|StartCameraFade :self (Game|GetPlayerCameraManager 0) :ToAlpha 1.0 :Duration 2.0 :bShouldFadeAudio true :bHoldWhenFinished true)
        (Utilities|FlowControl|Delay 2.0)
        (Variables|/Game/PhysicalWaterSurface/Blueprints/Buoyancy.Buoyancy_C|SetEnableBuoyancy _buoyancy true)
        (Transformation|SetActorLocation _self_2 (Math|Vector|MakeVector (.x _returnvalue_3) (.y _returnvalue_3) 0.0) false true)
        (Utilities|FlowControl|Delay 2.0)
        (CameraFades|StartCameraFade :self (Game|GetPlayerCameraManager 0) :FromAlpha 1.0 :Duration 2.0 :bShouldFadeAudio true :bHoldWhenFinished true)
        (Variables|Default|SetisEnableUpDown true)
        (Rendering|Material|SetScalarParameterValue (Variables|Default|GetSubMatInstance) "EmissiveValue" 0.0 :!class /Script/Engine.MaterialInstanceDynamic)))))

(event Custom|AimMode
  (params (isAim :type Boolean))
  (bind _returnvalue (Game|GetPlayerController 0))
  (bind _aimcamera (Variables|Default|GetAimCamera))
  (bind _maincamera (Variables|Default|GetMainCamera))
  (bind _returnvalue_2 (HUD|GetHUD _returnvalue))
  ;[1 1 1] 瞄准模式
  (bind _output_get (Variables|Default|SetisAim isAim))
  (if _output_get
    (Components|Activation|Deactivate _maincamera)
    (Components|Activation|Activate _aimcamera false)
    (Variables|Default|SetisEnableUpDown false)
    (bind _assubmarine_hud (Utilities|Casting|CastToSubmarineHUD _returnvalue_2))
    (Default|AddAim _assubmarine_hud)
    (else
      (Components|Activation|Deactivate _aimcamera)
      (Components|Activation|Activate _maincamera false)
      (Variables|Default|SetisEnableUpDown true)
      (bind _assubmarine_hud_2 (Utilities|Casting|CastToSubmarineHUD _returnvalue_2))
      (Default|RemoveAim _assubmarine_hud_2))))

(event Custom|MoveForward
  (bind _floatingpawnmovement (Variables|Default|GetFloatingPawnMovement))
  ;[1 1 1] 沉没测试
  (if (Variables|Default|GetisSunk)
    (Class|PawnMovementComponent|AddInputVector _floatingpawnmovement "0.000000,0.000000,-1.000000" true)
    (else
      (Class|PawnMovementComponent|AddInputVector _floatingpawnmovement (Transformation|GetActorForwardVector self) true)
      (Variables|/Script/Engine.FloatingPawnMovement|SetMaxSpeed (Variables|Default|GetFloatingPawnMovement) 2.5e+03))))

(event Custom|FireMissle
  (params (NewParam :type Boolean))
  (bind _firepoint (Variables|Default|GetFirePoint))
  (bind _returnvalue (Transformation|GetWorldTransform _firepoint))
  ;[1 1 1] 发射鱼雷导弹
  (if (== (Game|Player|GetPlayerPawn 0) self)
    (bind _outactors (Actor|GetAllActorsOfClass "/Game/Blueprints/Ships/Ship.Ship_C"))
    (if (Utilities|IsValid (Utilities|Array|Get(acopy) _outactors))
      (if (> (Variables|/Game/Blueprints/Ships/Ship.Ship_C|GetHealth (Utilities|Array|Get(acopy) _outactors)) 0)
        (bind _returnvalue_2 (Game|SpawnActorfromClass "/Game/Blueprints/Ships/Missile.Missile_C" (Math|Transform|MakeTransform (.location _returnvalue) (.rotation _returnvalue) "1,1,1") "Undefined" 0 0))
        (Default|FireIt _returnvalue_2 "0, 0, 0" "0, 0, 0" (Utilities|Array|Get(acopy) _outactors))))))

(event EventTick
  (params (DeltaSeconds :type Float%20%28single-precision%29))
  ;[1 1 1] 1. 向前机动
  ; 2. 转向功能
  ; 3. 水深检测
  (Variables|Default|SetDeltaSeconds DeltaSeconds)
  (CallFunction|MoveForward)
  (bind _isrightdec (CallFunction|CheckRotation))
  (Class|Actor|AddActorWorldRotation self (Math|Rotator|MakeRotator 0.0 0.0 (* (* (Variables|Default|GetRotateSpeed) (Variables|Default|GetDeltaSeconds)) _isrightdec)))
  (CallFunction|HeightCheck))

(event EventBeginPlay
  (bind _assubmarine_game_mode (Utilities|Casting|CastToSubmarineGameMode (Game|GetGameMode)))
  (Variables|/Game/Blueprints/GameFrame/SubmarineGameMode.SubmarineGameMode_C|SetMainSubmarine _assubmarine_game_mode self))

(event Input|AxisEvents|InputAxisMoveRight
  (params (AxisValue :type Float%20%28single-precision%29))
  (Pawn|Input|AddControllerYawInput AxisValue))

(event Input|AxisEvents|InputAxisMoveUp
  (params (AxisValue :type Float%20%28single-precision%29))
  (Pawn|Input|AddControllerPitchInput AxisValue))

(fn ConstructionScript
  (bind _returnvalue (Rendering|Material|CreateDynamicMaterialInstance (Variables|Default|GetSK_Submarine) 0 (Rendering|Material|GetMaterial (Variables|Default|GetSK_Submarine) 0) :!class /Script/Engine.PrimitiveComponent))
  (Variables|Default|SetSubMatInstance _returnvalue))

(fn CheckRotation
  (bind _out360 (CallFunction|Trans180to360 (.yaw (Transformation|GetWorldRotation (Variables|Default|GetMainCamera)))))
  (LocalVariables|SetCameraRotZ _out360)
  (bind _out360_2 (CallFunction|Trans180to360 (.yaw (Transformation|GetWorldRotation (Variables|Default|GetStaticMesh)))))
  (LocalVariables|SetSelfRotZ _out360_2)
  (if (> (Math|Float|Absolute(Float) (- (Math|Float|Absolute(Float) (LocalVariables|GetCameraRotZ)) (Math|Float|Absolute(Float) (LocalVariables|GetSelfRotZ)))) 1e+01)
    (if (< (LocalVariables|GetCameraRotZ) 1.8e+02)
      (LocalVariables|SetisRightD (not (Math|Float|InRange(Float) (LocalVariables|GetSelfRotZ) (LocalVariables|GetCameraRotZ) (+ (LocalVariables|GetCameraRotZ) 1.8e+02))))
      (else
        (LocalVariables|SetisRightD (Math|Float|InRange(Float) (LocalVariables|GetSelfRotZ) (- (LocalVariables|GetCameraRotZ) 1.8e+02) (LocalVariables|GetCameraRotZ)))))
    (if (LocalVariables|GetisRightD)
      (return 1.0)
      (else
        (return -1.0)))
    (else
      (return 0.0))))

(fn Trans180to360
  (params (IN180 :type Float%20%28single-precision%29))
  (if (< IN180 0.0)
    (return (+ IN180 3.6e+02))
    (else
      (return IN180))))

(fn HeightCheck
  (bind _self self)
  (bind _returnvalue (Transformation|GetActorLocation _self))
  (bind _returnvalue_2 (+ (.z _returnvalue) 7.2e+02))
  (bind _returnvalue_3 (/ _returnvalue_2 1e+02))
  (bind _returnvalue_4 (Math|Float|Truncate _returnvalue_3))
  (if (> _returnvalue_4 0)
    (Variables|Default|SetHeight 0)
    (else
      (Variables|Default|SetHeight _returnvalue_4))))