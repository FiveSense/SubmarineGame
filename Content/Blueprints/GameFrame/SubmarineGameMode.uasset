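; Submarine game mode that switches the player's view by possessing a different pawn: the submarine, a missile, or a ship.
; ChangeCamera possesses the new missile or ship, and a ship view returns to the submarine after a delay.
; BackToSubmarine re-possesses the first SubmarinePawn found in the level.
; Released pawns get a default controller spawned so they stay controlled.
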(event Custom|ChangeCamera
  (params (NewCamera :type E_Camera%20Enum) (NewPawn :type Pawn%20Object%20Reference) (OldPawn :type Pawn%20Object%20Reference) (Delay :type Float%20%28single-precision%29))
  (bind _returnvalue (Game|GetPlayerController 0))
  ;[1 1 1] 切换摄像机（切换pawn）
  (Variables|Default|SetOldTempPawn OldPawn)
  (Utilities|FlowControl|Sequence
    (:then_0
      (switch Utilities|FlowControl|Switch|SwitchonE_Camera NewCamera
        (:NewEnumerator0
          (CallFunction|BacktoSubmarine OldPawn))
        (:NewEnumerator1
          (bind _asmissile (Utilities|Casting|CastToMissile NewPawn))
          (Pawn|Possess _returnvalue _asmissile))
        (:NewEnumerator2
          (bind _asship (Utilities|Casting|CastToShip NewPawn))
          (Pawn|Possess _returnvalue _asship)
          (Variables|Default|SetOldTempPawn _asship)
          (Utilities|FlowControl|Delay Delay)
          (CallFunction|BacktoSubmarine _asship))))
    (:then_1
      (Pawn|SpawnDefaultController OldPawn))))

(event Custom|BackToSubmarine
  (params (OldPawn :type Pawn%20Object%20Reference))
  ;[1 1 1] 控制潜艇
  (bind _outactors (Actor|GetAllActorsOfClass "/Game/Blueprints/GameFrame/SubmarinePawn.SubmarinePawn_C"))
  (Pawn|Possess (Game|GetPlayerController 0) (Utilities|Array|Get(acopy) _outactors))
  (Pawn|SpawnDefaultController OldPawn))

(event EventBeginPlay)

(fn ConstructionScript)