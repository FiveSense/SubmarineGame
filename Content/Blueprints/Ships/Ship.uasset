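; Ship pawn that sails forward on buoyancy and floating movement, then stops and sinks as it takes damage.
; Tick drives movement and tilt from a small integer Health state.
; Damage applies burn/dissolve through dynamic materials, and death disables buoyancy, then destroys the actor after a delay.
; Explode passes a random arrow location to an empty CreateParticle, while MakeExplose, which spawns the emitters, is not called here.
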(event Custom|Damage
  (params (damage :type Integer))
  (Variables|Default|SetHealth (- (Variables|Default|GetHealth) damage))
  (switch int (Variables|Default|GetHealth)
    (:Default
      (Variables|Default|SetHealth 0 :!label _label)
      (CallFunction|BreakDown 0.4 "(R=0.364706,G=0.007843,B=0.007843,A=1.000000)" 3.0 "(R=0.580392,G=0.215686,B=0.000000,A=1.000000)")
      (CallFunction|Explode (Math|Random|RandomIntegerinRange 0 2))
      (CallFunction|Sunk)
      (Utilities|FlowControl|Delay 8.0)
      (for _array_element (Variables|Default|GetPar1)
        (Utilities|IsValid _array_element
          (:Is%20Valid
            (Components|DestroyComponent _array_element))))
      (Actor|DestroyActor))
    (:0
      (goto _label))
    (:1
      (Variables|Default|SetHealth 1)
      (CallFunction|BreakDown 0.1 "(R=0.364706,G=0.007843,B=0.007843,A=1.000000)" 3.0 "(R=0.580392,G=0.215686,B=0.000000,A=1.000000)")
      (CallFunction|Explode (Math|Random|RandomIntegerinRange 0 2)))))

(event Custom|Sunk
  (bind _floatingpawnmovement (Variables|Default|GetFloatingPawnMovement))
  (Class|PawnMovementComponent|AddInputVector _floatingpawnmovement "0.000000,0.000000,-1.000000" true)
  (Variables|/Script/Engine.FloatingPawnMovement|SetMaxSpeed _floatingpawnmovement 1e+03)
  (Variables|/Game/PhysicalWaterSurface/Blueprints/Buoyancy.Buoyancy_C|SetEnableBuoyancy (Variables|Default|GetBuoyancy) false))

(event Custom|Explode
  (params (position :type Integer))
  (switch int position
    (:0
      (CallFunction|CreateParticle (Transformation|GetWorldLocation (Variables|Default|GetArrowFront))))
    (:1
      (CallFunction|CreateParticle (Transformation|GetWorldLocation (Variables|Default|GetArrowMiddle))))
    (:2
      (CallFunction|CreateParticle (Transformation|GetWorldLocation (Variables|Default|GetArrowBack))))))

(event Custom|MakeExplose
  (params (Location :type Vector))
  (Utilities|FlowControl|Sequence
    (:then_0
      (bind _returnvalue (Effects|SpawnEmitteratLocation "/Game/Explosions/Particles/P_Destruction1.P_Destruction1" Location "0, 0, 0" false))
      (Transformation|SetWorldScale3D _returnvalue "20.000000,20.000000,20.000000")
      (Utilities|Array|Add (Variables|Default|GetPar1) _returnvalue))
    (:then_1
      (bind _returnvalue_2 (Effects|SpawnEmitteratLocation "/Game/Explosions/Particles/P_ImpactExplosion3.P_ImpactExplosion3" Location "0, 0, 0" false))
      (Transformation|SetWorldScale3D _returnvalue_2 "20.000000,20.000000,20.000000")
      (Utilities|Array|Add (Variables|Default|GetPar1) _returnvalue_2))
    (:then_2
      (bind _returnvalue_3 (Effects|SpawnEmitteratLocation "/Game/Explosions/Particles/P_Explode2.P_Explode2" Location "0, 0, 0" false))
      (Transformation|SetWorldScale3D _returnvalue_3 "20.000000,20.000000,20.000000")
      (Utilities|Array|Add (Variables|Default|GetPar1) _returnvalue_3))))

(event EventBeginPlay)

(event EventTick
  (params (DeltaSeconds :type Float%20%28single-precision%29))
  (bind _floatingpawnmovement (Variables|Default|GetFloatingPawnMovement))
  ;[1 1 1] 航行
  (switch int (Variables|Default|GetHealth)
    (:Default
      (Variables|Default|SetisDead true :!label _label))
    (:0
      (Class|Actor|AddActorWorldRotation self "0.000000, 0,-0.100000")
      (goto _label))
    (:1
      (Variables|/Script/Engine.FloatingPawnMovement|SetMaxSpeed _floatingpawnmovement 0.0))
    (:2
      (Class|PawnMovementComponent|AddInputVector _floatingpawnmovement "1.000000,0.000000,0.000000" true)
      (Variables|/Script/Engine.FloatingPawnMovement|SetMaxSpeed _floatingpawnmovement 2.5e+03))))

(fn ConstructionScript
  (CallFunction|BreakDown -1.0 "(R=1.000000,G=1.000000,B=1.000000,A=1.000000)" 1.0 "(R=0.580392,G=0.215686,B=0.000000,A=1.000000)"))

(fn BreakDown
  (params (Dissolve :type Float%20%28single-precision%29) (ColorMultiplier :type Linear%20Color%20Structure) (RoughnessMultiplier :type Float%20%28single-precision%29) (DissolveColor :type Linear%20Color%20Structure))
  (bind _staticmesh (Variables|Default|GetStaticMesh))
  (for (_array_element _array_index) (Rendering|Material|GetMaterials _staticmesh)
    (bind _returnvalue (Rendering|Material|CreateDynamicMaterialInstance _staticmesh _array_index _array_element :!class /Script/Engine.PrimitiveComponent))
    (Rendering|Material|SetScalarParameterValue _returnvalue "Dissolve" Dissolve :!class /Script/Engine.MaterialInstanceDynamic)
    (Rendering|Material|SetVectorParameterValue _returnvalue "ColorMultiplier" ColorMultiplier :!class /Script/Engine.MaterialInstanceDynamic)
    (Rendering|Material|SetScalarParameterValue _returnvalue "RoughnessMultiplier" RoughnessMultiplier :!class /Script/Engine.MaterialInstanceDynamic)
    (Rendering|Material|SetVectorParameterValue _returnvalue "DissolveColor" DissolveColor :!class /Script/Engine.MaterialInstanceDynamic)))

(fn CreateParticle
  (params (Location :type Vector)))